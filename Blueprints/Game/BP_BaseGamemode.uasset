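; Base game mode that handles character death and player spawning at game player starts.
; CharacterDead broadcasts the victim and instigator, then, if AutoRespawn is on, launches a respawn timer on the victim's BP_PlayerController.
; SpawnPlayer picks a random free BP_GamePlayerStart and delegates the spawn to it, with no fallback when none are free.
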(fn `CharacterDead`
  (params (DeadCharter :type "/Game/Blueprints/Player/BP_PlayerCharacter Object Reference") (DeathInstigator :type "/Game/Blueprints/Player/BP_PlayerController Object Reference"))
  (`self.CharDead` DeadCharter DeathInstigator)
  (bind _asbp_player_controller (cast `/Game/Blueprints/Player/BP_PlayerController` (`Pawn.GetController` DeadCharter)))
  (if (`self.AutoRespawn`)
    (`/Game/Blueprints/Player/BP_PlayerController.LaunchRespawnTimer` _asbp_player_controller (`self.RespawnTime`))))

(fn `GetFreeSpawnPoints`
  (returns (FreeSpawn :type "Array of /Game/Blueprints/Game/BP_GamePlayerStart Object Reference"))
  (locals (L_FreePoints :type "Array of /Game/Blueprints/Game/BP_GamePlayerStart Object Reference"))
  (bind _outactors (`GameplayStatics.GetAllActorsOfClass` "/Game/Blueprints/Game/BP_GamePlayerStart.BP_GamePlayerStart_C"))
  (for _array_element _outactors
    (if (`/Game/Blueprints/Game/BP_GamePlayerStart.IsFree` _array_element)
      (`KismetArrayLibrary.Array_Add` (`local.L_FreePoints`) _array_element)))
  (return (`local.L_FreePoints`)))

(fn `SpawnPlayer`
  (params (Player :type "/Game/Blueprints/Player/BP_PlayerController Object Reference"))
  (locals (L_PlayerStart :type "/Game/Blueprints/Game/BP_GamePlayerStart Object Reference"))
  (bind _freespawn (`self.GetFreeSpawnPoints`))
  (bind _output_get (set `local.L_PlayerStart` (`|GetArrayItem` _freespawn (`KismetMathLibrary.RandomInteger` (`KismetArrayLibrary.Array_LastIndex` _freespawn)))))
  (`/Game/Blueprints/Game/BP_GamePlayerStart.SpawnCharter` _output_get Player))

(fn `UserConstructionScript`)