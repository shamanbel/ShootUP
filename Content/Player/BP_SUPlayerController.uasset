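; BP_SUPlayerController is the player controller that handles the in-game text chat.
; On BeginPlay, a local controller clears existing widgets and adds WBP_PlayerHUD, which holds the chat window.
; GetChatMessage pairs the text with the player's name and loops over the game mode's AllPlayerControllers, calling UpdateChat on each to refresh its chat widget.
; The T key toggles the mouse cursor.
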(event `self.ReceiveBeginPlay`
  (if (`self.IsLocalController`)
    (`WidgetLayoutLibrary.RemoveAllWidgets`)
    (`self.SetupChatWindow`)))

(event `SetupChatWindow`
  ;[1 1 1] Создание окна чата в игре
  (bind _returnvalue (`|CreateWidget` "/Game/UI_Single/WBP_PlayerHUD.WBP_PlayerHUD_C"))
  (bind _output_get (set `self.GamePlayChatWB` _returnvalue))
  (`UserWidget.AddToViewport` _output_get 0))

(event `GetChatMessage`
  (params (TextToSend :type Text))
  ;[1 1 1] Сообщение  об обновлении чата
  (set `self.SenderText` TextToSend)
  (set `self.SenderName` (`KismetTextLibrary.Conv_StringToText` (`AdvancedSessionsLibrary.GetPlayerName` self)))
  (bind _asbp_sugame_mode_base (cast `/Game/BP_SUGameModeBase` (`GameplayStatics.GetGameMode`)))
  (for _array_element (`/Game/BP_SUGameModeBase.AllPlayerControllers` _asbp_sugame_mode_base)
    (bind _asbp_suplayer_controller (cast `/Game/Player/BP_SUPlayerController` _array_element))
    (`self.UpdateChat` _asbp_suplayer_controller (`self.SenderName`) (`self.SenderText`))))

(event `UpdateChat`
  (params (SenderName :type Text) (SenderText :type Text))
  (`/Game/UI/AllLevels/ChatWindow.UpdateChatWindow` (`/Game/UI_Single/WBP_PlayerHUD.GamePlayChat` (`self.GamePlayChatWB`)) SenderName SenderText))

(event `Key|T`
  (params (Key :type "Key Structure"))
  (:`Pressed`
    (`/Engine/EditorBlueprintResources/StandardMacros.FlipFlop`
      (:`A`
        (set `self.bShowMouseCursor` true))
      (:`B`
        (set `self.bShowMouseCursor` false)))))

(fn `UserConstructionScript`)